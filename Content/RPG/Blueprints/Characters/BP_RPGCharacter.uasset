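; RPG character Blueprint with modular body meshes, weapon equipping and the main UI.
; The construction script makes body-part meshes follow the main Mesh pose and registers chest, legs and feet slots with default meshes.
; BeginPlay creates UI_Main with mouse input, and I, E and C toggle its inventory, equipment and crafting panels.
; EquipWeapon spawns and socket-attaches a weapon to HandsR, or destroys it when given no valid class, updating AxeEquipped.
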(event `self.ReceiveBeginPlay`
  (bind _returnvalue (`GameplayStatics.GetPlayerController` 0))
  (`|ExecutionSequence`
    (:`then_0`
      (bind _returnvalue_2 (`|CreateWidget` "/Game/RPG/UI/UI_Main.UI_Main_C" _returnvalue))
      (bind _output_get (set `self.Main` _returnvalue_2))
      (`UserWidget.AddToViewport` _output_get 0)
      (`WidgetBlueprintLibrary.SetInputMode_GameAndUIEx` _returnvalue _output_get)
      (set `PlayerController.bShowMouseCursor` true _returnvalue))))

(event `self.EquipWeapon`
  (params (WeaponClass :type "WeaponBase Class Reference") (WeaponSocket :type Name))
  (bind _weapon (`self.Weapon`))
  (if (`KismetSystemLibrary.IsValidClass` WeaponClass)
    (bind _returnvalue (`|SpawnActorFromClass` WeaponClass (`KismetMathLibrary.MakeTransform` (0.0 0.0 0.0)) "Undefined" "OverrideRootScale" null null))
    (`self.K2_AttachToComponent` _returnvalue (`self.Hands_R`) WeaponSocket "SnapToTarget" "SnapToTarget" "SnapToTarget" true)
    (set `self.Weapon` _returnvalue)
    (set `self.bAxeEquipped` true)
    (else
      (`/Engine/EditorBlueprintResources/StandardMacros.IsValid` _weapon
        (:`Is Valid`
          (`self.K2_DestroyActor` _weapon)
          (set `self.Weapon` null)
          (set `self.bAxeEquipped` false))))))

(event `Key|I`
  (params (Key :type "Key Structure"))
  (:`Pressed`
    (`/Game/Assets/UI/SpaceGUI/blueprints/bc_gui_functions.GUI Toggle Widget` (`/Game/RPG/UI/UI_Main.W_Inventory` (`self.Main`)))))

(event `Key|E`
  (params (Key :type "Key Structure"))
  (:`Pressed`
    (`/Game/Assets/UI/SpaceGUI/blueprints/bc_gui_functions.GUI Toggle Widget` (`/Game/RPG/UI/UI_Main.W_Equipment` (`self.Main`)))))

(event `Key|C`
  (params (Key :type "Key Structure"))
  (:`Pressed`
    (`/Game/Assets/UI/SpaceGUI/blueprints/bc_gui_functions.GUI Toggle Widget` (`/Game/RPG/UI/UI_Main.W_Crafting` (`self.Main`)))))

(fn `UserConstructionScript`
  (`|ExecutionSequence`
    (:`then_0`
      (`SkinnedMeshComponent.SetLeaderPoseComponent` (`self.Hair`) (`self.Mesh`) false false)
      (`SkinnedMeshComponent.SetLeaderPoseComponent` (`self.Body`) (`self.Mesh`) false false)
      (`SkinnedMeshComponent.SetLeaderPoseComponent` (`self.Legs`) (`self.Mesh`) false false)
      (`SkinnedMeshComponent.SetLeaderPoseComponent` (`self.Feet`) (`self.Mesh`) false false)
      (`SkinnedMeshComponent.SetLeaderPoseComponent` (`self.Hands_L`) (`self.Mesh`) false false)
      (`SkinnedMeshComponent.SetLeaderPoseComponent` (`self.Hands_R`) (`self.Mesh`) false false))
    (:`then_1`
      (`self.AddSKMToMap` "EES_Chest" (make `SKMData` (`self.Body`) "/Game/Assets/3D/Characters/Warrior/Meshes/Characters/Separates/Bodies/TopBodies/SK_TopBody_A.SK_TopBody_A"))
      (`self.AddSKMToMap` "EES_Legs" (make `SKMData` (`self.Legs`) "/Game/Assets/3D/Characters/Warrior/Meshes/Characters/Separates/Bodies/BotBodies/SK_BotBody_A.SK_BotBody_A"))
      (`self.AddSKMToMap` "EES_Feet" (make `SKMData` (`self.Feet`) "/Game/Assets/3D/Characters/Warrior/Meshes/Characters/Separates/Bodies/Boots/SK_BootsS1.SK_BootsS1")))))